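; Invisible ball actor for a paddle game, launched by a physics force derived from its Speed variable when play begins.
; It destroys itself when it hits an enemy paddle or when Tick finds its sphere outside fixed world X bounds on either side.
; A Space Bar press toggles the visibility of the sphere and its children.
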(event EventBeginPlay
  (Physics|AddForce :Force (Math|Conversions|ToVector(Float) (Variables|Default|Getspeed))))

(event Collision|EventActorBeginOverlap
  (params (OtherActor :type Actor%20Object%20Reference)))

(event Collision|EventHit
  (params (MyComp :type Primitive%20Component%20Object%20Reference) (Other :type Actor%20Object%20Reference) (OtherComp :type Primitive%20Component%20Object%20Reference) (bSelfMoved :type Boolean) (HitLocation :type Vector :default "0, 0, 0") (HitNormal :type Vector :default "0, 0, 0") (NormalImpulse :type Vector :default "0, 0, 0") (Hit :type Hit%20Result%20Structure%20%28by%20ref%29))
  (Utilities|Casting|CastTobp_EnemyPaddle Other)
  (Actor|DestroyActor))

(event EventTick
  (params (DeltaSeconds :type Float%20%28single-precision%29))
  (bind _sphere (Variables|Default|GetSphere))
  (bind _returnvalue (Transformation|GetWorldLocation _sphere))
  (if (<= (.x _returnvalue) -1e+03)
    (Actor|DestroyActor :!label _label)
    (elif (>= (.x _returnvalue) 1e+03)
      (goto _label))))

(event Input|KeyboardEvents|SpaceBar
  (params (Key :type Key%20Structure :default "None"))
  (:Pressed
    (Rendering|ToggleVisibility (Variables|Default|GetSphere) true)))

(fn ConstructionScript)