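; Player paddle Actor that moves vertically on the Z axis from player input, within fixed bounds.
; Each Tick offsets the Cube component locally by an input axis key value scaled by Speed and delta time.
; It then checks the actor's Z location and snaps it back to symmetric upper or lower limits when exceeded.
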(event EventBeginPlay
  (|CallParentFunction))

(event Collision|EventActorBeginOverlap
  (params (OtherActor :type Actor%20Object%20Reference))
  (|CallParentFunction OtherActor) ; This node is disabled and will not be called.\nDrag off pins to build functionality.
)

(event EventTick
  (params (DeltaSeconds :type Float%20%28single-precision%29))
  (bind _returnvalue (Transformation|GetActorLocation))
  (|CallParentFunction DeltaSeconds)
  (Transformation|AddLocalOffset (Variables|Default|GetCube) (Math|Vector|MakeVector 0.0 0.0 (* (Class|Actor|GetInputAxisKeyValue) (Variables|Default|Getspeed) DeltaSeconds)) false false)
  (if (> (.z _returnvalue) 6.3e+02)
    (Transformation|SetActorLocation (Math|Vector|MakeVector (.x _returnvalue) (.y _returnvalue) 6.3e+02) false false)
    (elif (< (.z _returnvalue) -6.3e+02)
      (Transformation|SetActorLocation (Math|Vector|MakeVector (.x _returnvalue) (.y _returnvalue) -6.3e+02) false false))))

(fn ConstructionScript
  (|CallParentFunction))