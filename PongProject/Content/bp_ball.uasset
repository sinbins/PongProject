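; Physics-driven ball for a paddle game, launched along negative X by an impulse on its Sphere when play begins.
; Tick watches the X position and, past either boundary, asks the Bp_ballSpawner for a new ball and destroys this one.
; Hitting a bp_playerPaddle spawns a Bp_InvisibleBall from the Sphere's transform at double the ball's velocity, so it travels ahead of the real ball.
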(event EventBeginPlay
  (Physics|AddImpulse (Variables|Default|GetSphere) "-10000.000000,0.000000,0.000000" "None" false))

(event Collision|EventActorBeginOverlap
  (params (OtherActor :type Actor%20Object%20Reference)))

(event EventTick
  (params (DeltaSeconds :type Float%20%28single-precision%29))
  (bind _sphere (Variables|Default|GetSphere))
  (bind _returnvalue (Transformation|GetWorldLocation _sphere))
  (if (<= (.x _returnvalue) -1e+03)
    (bind _returnvalue_2 (Actor|GetActorOfClass "/Game/bp_ballSpawner.bp_ballSpawner_C" :!label _label))
    (Default|SpawnBall _returnvalue_2)
    (Actor|DestroyActor)
    (elif (>= (.x _returnvalue) 1e+03)
      (goto _label))))

(event Collision|EventHit
  (params (MyComp :type Primitive%20Component%20Object%20Reference) (Other :type Actor%20Object%20Reference) (OtherComp :type Primitive%20Component%20Object%20Reference) (bSelfMoved :type Boolean) (HitLocation :type Vector :default "0, 0, 0") (HitNormal :type Vector :default "0, 0, 0") (NormalImpulse :type Vector :default "0, 0, 0") (Hit :type Hit%20Result%20Structure%20%28by%20ref%29))
  (bind _sphere (Variables|Default|GetSphere))
  (Utilities|Casting|CastTobp_playerPaddle Other)
  (bind _returnvalue (Game|SpawnActorfromClass "/Game/bp_InvisibleBall.bp_InvisibleBall_C" (Transformation|GetRelativeTransform _sphere) "Undefined" "MultiplyWithRoot" 0 0))
  (Class|PrimitiveComponent|SetAllPhysicsLinearVelocity (Variables|/Game/bp_InvisibleBall.bp_InvisibleBall_C|GetSphere _returnvalue) (* (Transformation|GetComponentVelocity _sphere) "2.000000,2.000000,2.000000") false))

(fn ConstructionScript)